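; Lobby player state that holds a player's replicated user name and exposes it to the lobby HUD.
; On BeginPlay it registers itself with the first player controller's BP_LobbyHud, retrying on a short timer until that HUD exists.
; SetName writes the name, and its RepNotify broadcasts the ChangeUserName dispatcher and prints a debug message.
; The same dispatcher also fires when the player state is destroyed.
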(event `self.ReceiveBeginPlay`
  (`self.TryBind`))

(event `self.ReceiveDestroyed`
  (`self.EventDispatcher_ChangeUserName` (`self.UserName`)))

(fn `OnRep_UserName`
  (bind _username (`self.UserName`))
  (`self.EventDispatcher_ChangeUserName` _username)
  (`KismetSystemLibrary.PrintString` (`KismetStringLibrary.Concat_StrStr` "On Rep User Name - " _username) true true (struct :`G` 1.0 :`B` 0.57625 :`A` 1.0) 10.0))

(fn `SetName`
  (params (UserName :type String))
  (set `self.UserName` UserName))

(fn `TryBind`
  (bind _asbp_lobby_hud (cast `/Game/_Game/BP_LobbyHud` (`PlayerController.GetHUD` (`GameplayStatics.GetPlayerController` 0)))
    (:`then`
      (`/Game/_Game/BP_LobbyHud.BindPlayerState` _asbp_lobby_hud self))
    (:`CastFailed`
      (`KismetSystemLibrary.K2_SetTimer` null "TryBind" 0.1))))

(fn `UserConstructionScript`)