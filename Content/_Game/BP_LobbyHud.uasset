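; Lobby HUD Blueprint that shows the lobby widget and keeps its player list in sync with user names.
; BeginPlay creates WBP_LobbyWidget, adds it to the viewport and switches to UI-only input with a visible cursor.
; BindPlayerState subscribes to a player state's user-name change dispatcher and immediately requests a list refresh.
; If the widget is not yet valid, a 0.1-second retry timer defers the refresh until it exists.
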(event `self.ReceiveBeginPlay`
  (bind _returnvalue (`GameplayStatics.GetPlayerController` 0))
  (bind _returnvalue_2 (`|CreateWidget` "/Game/_Game/UI/WBP_LobbyWidget.WBP_LobbyWidget_C"))
  (bind _output_get (set `self.HudWidget` _returnvalue_2))
  (`UserWidget.AddToViewport` _output_get 0)
  (`WidgetBlueprintLibrary.SetInputMode_UIOnlyEx` _returnvalue null)
  (set `PlayerController.bShowMouseCursor` true _returnvalue))

(fn `BindPlayerState`
  (params (PlayerState :type "/Game/_Game/BP_LobbyPlayerState Object Reference"))
  (add `/Game/_Game/BP_LobbyPlayerState.EventDispatcher_ChangeUserName` PlayerState (`|CreateDelegate` :!event `UpdateUserName`))
  (`KismetSystemLibrary.PrintString` "Bind Player State Complate!!!" true true (struct :`G` 0.66 :`B` 1.0 :`A` 1.0) 60.0)
  (`self.UpdateUserName` ""))

(fn `UpdateUserName`
  (params (UserName :type String))
  (bind _hudwidget (`self.HudWidget`))
  (`/Engine/EditorBlueprintResources/StandardMacros.IsValid` _hudwidget
    (:`Is Valid`
      (`/Game/_Game/UI/WBP_LobbyWidget.UpadatePlayerList` _hudwidget))
    (:`Is Not Valid`
      (if (not (`KismetSystemLibrary.K2_TimerExists` null "WaitCreateHudWidget"))
        (`KismetSystemLibrary.K2_SetTimer` null "WaitCreateHudWidget" 0.1)))))

(fn `UserConstructionScript`)

(fn `WaitCreateHudWidget`
  (bind _hudwidget (`self.HudWidget`))
  (`/Engine/EditorBlueprintResources/StandardMacros.IsValid` _hudwidget
    (:`Is Valid`
      (`/Game/_Game/UI/WBP_LobbyWidget.UpadatePlayerList` _hudwidget))
    (:`Is Not Valid`
      (`KismetSystemLibrary.K2_SetTimer` null "WaitCreateHudWidget" 0.1))))