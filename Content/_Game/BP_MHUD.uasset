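; BP_MHUD is a HUD Blueprint that sets up the sub-game widget and relays refresh requests to the possessions UI.
; On BeginPlay it adds WBP_SubGameWidget to the viewport collapsed and switches the first player controller to Game and UI input.
; It caches PossessionWidget as WBP_Possessions, retrying on a short timer until that widget is valid.
; UpdatePossessionUI calls UpdatePossession on the cached widget.
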(event `self.ReceiveBeginPlay`
  (bind _returnvalue (`GameplayStatics.GetPlayerController` 0))
  (`parent.ReceiveBeginPlay`)
  (`self.Bind WBP Possession`)
  (bind _returnvalue_2 (`|CreateWidget` "/Game/_Game/UI/WBP_SubGameWidget.WBP_SubGameWidget_C" _returnvalue))
  (bind _output_get (set `self.SubGameWidget` _returnvalue_2))
  (`UserWidget.AddToViewport` _output_get 0)
  (`WidgetBlueprintLibrary.SetInputMode_GameAndUIEx` _returnvalue null)
  (`Widget.SetVisibility` (`self.SubGameWidget`) "Collapsed"))

(event `self.UpdatePossessionUI`
  (`/Game/_Game/UI/WBP_Possessions.UpdatePossession` (`self.As WBP Possessions`)))

(fn `Bind WBP Possession`
  (bind _possessionwidget (`self.PossessionWidget`))
  (`/Engine/EditorBlueprintResources/StandardMacros.IsValid` _possessionwidget
    (:`Is Valid`
      (bind _aswbp_possessions (cast `/Game/_Game/UI/WBP_Possessions` _possessionwidget))
      (set `self.As WBP Possessions` _aswbp_possessions))
    (:`Is Not Valid`
      (`KismetSystemLibrary.K2_SetTimer` null "Bind WBP Possession" 0.1))))

(fn `UserConstructionScript`)