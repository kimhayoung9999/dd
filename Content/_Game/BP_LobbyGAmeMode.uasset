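; Lobby GameMode Blueprint that traces the player join flow with on-screen debug messages.
; BeginPlay prints a long-lived startup message.
; HandleStartingNewPlayer and PostLogin call their parent implementations, then print the joining player controller's display name.
; It contains no other lobby logic.
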(event `self.ReceiveBeginPlay`
  (`KismetSystemLibrary.PrintString` "LobbyGameMode BeginPlay" true true (struct :`G` 0.66 :`B` 1.0 :`A` 1.0) 60.0))

(event `self.HandleStartingNewPlayer`
  (params (NewPlayer :type "PlayerController Object Reference"))
  (`parent.HandleStartingNewPlayer` NewPlayer)
  (`KismetSystemLibrary.PrintString` (`KismetStringLibrary.Concat_StrStr` "Handle Starting New Player - " (`KismetSystemLibrary.GetDisplayName` NewPlayer)) true true (struct :`R` 1.0 :`B` 0.394548 :`A` 1.0) 10.0))

(event `self.K2_PostLogin`
  (params (NewPlayer :type "PlayerController Object Reference"))
  (`parent.K2_PostLogin` NewPlayer)
  (`KismetSystemLibrary.PrintString` (`KismetStringLibrary.Concat_StrStr` "OnPostLogin New Player - " (`KismetSystemLibrary.GetDisplayName` NewPlayer)) true true (struct :`G` 0.66 :`B` 1.0 :`A` 1.0) 10.0))

(fn `UserConstructionScript`)