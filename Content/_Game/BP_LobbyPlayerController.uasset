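; BP_LobbyPlayerController is the lobby player controller that passes the player's name from the game instance to the lobby player state.
; On possess it logs the pawn and calls ResClientPossess, which by its name is the client response.
; That event reads PlayerName from BP_MGameInstance and sends it through ReqChangeName, a server request that calls SetName on BP_LobbyPlayerState.
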(event `self.ReceivePossess`
  (params (PossessedPawn :type "Pawn Object Reference"))
  (`KismetSystemLibrary.PrintString` (`KismetStringLibrary.Concat_StrStr` "Possessed Pawn - " (`KismetSystemLibrary.GetDisplayName` PossessedPawn)))
  (`self.ResClientPossess`))

(event `ResClientPossess`
  (`KismetSystemLibrary.PrintString` "ResClientPossess")
  (bind _asbp_mgame_instance (cast `/Game/_Game/BP_MGameInstance` (`GameplayStatics.GetGameInstance`)))
  (`self.ReqChangeName` (`/Game/_Game/BP_MGameInstance.PlayerName` _asbp_mgame_instance)))

(event `ReqChangeName`
  (params (UserName :type String))
  ;[1 0 0] (Server) 이름 변경 요청
  (bind _asbp_lobby_player_state (cast `/Game/_Game/BP_LobbyPlayerState` (`self.PlayerState`)))
  (`/Game/_Game/BP_LobbyPlayerState.SetName` _asbp_lobby_player_state UserName))

(fn `UserConstructionScript`)